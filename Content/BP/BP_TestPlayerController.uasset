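; Test player controller that runs a charge-and-fire mechanic and switches between the HUD and a menu panel.
; BeginPlay adds the input mapping context and creates both widgets.
; Holding charge runs a looping timer that builds progress into whole charges up to a maximum; firing spends one, with HUD updates pushed directly.
; ShowPanel swaps widget visibility, input mode, mouse cursor and menu activation.
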(event `self.ReceiveBeginPlay`
  ; Event Begin Play
  (`EnhancedInputSubsystemInterface.AddMappingContext` (pcsubsystem `EnhancedInputLocalPlayerSubsystem` (`GameplayStatics.GetPlayerController` 0)) "/Game/Input/IMC_Test.IMC_Test" 0 (struct))
  (bind _returnvalue (`|CreateWidget` "/Game/UI/HUD/WBP_HUD.WBP_HUD_C" self))
  (bind _output_get (set `self.WBP_HUD` _returnvalue))
  (`UserWidget.AddToViewport` _output_get 0)
  (bind _returnvalue_2 (`|CreateWidget` "/Game/UI/ToggleButtonGroup/WBP_MainContent.WBP_MainContent_C"))
  (bind _output_get_2 (set `self.WBP_Menu` _returnvalue_2))
  (`UserWidget.AddToViewport` _output_get_2 0)
  (`self.ShowPanel` false))

(event `EnhancedInput|/Game/Input/Actions/IA_Fire`
  (params (ActionValue :type Boolean) (ElapsedSeconds :type "Float (double-precision)") (TriggeredSeconds :type "Float (double-precision)") (InputAction :type "InputAction Object Reference" :default "/Game/Input/Actions/IA_Fire.IA_Fire"))
  ; INPUTS
  (:`Started`
    (if (> (`self.CurrentFullyCharges`) 0)
      (if (>= (`self.CurrentFullyCharges`) 1)
        (set `self.CurrentFullyCharges` (`KismetMathLibrary.Clamp` (- (`self.CurrentFullyCharges`) 1) 0 3))
        (`/Game/UI/HUD/WBP_HUD.Shoot` (`self.WBP_HUD`))))))

(event `StartTimeEvent_Event`
  ; Event that  creates the timer event to refresh the charging
  (bind _returnvalue (`KismetSystemLibrary.K2_SetTimerDelegate` (delegate `ChargeProgressionUpdate_Event`) (`self.TicksPerChargeUpdate`) true))
  (set `self.ChargeTimerHandle` _returnvalue))

(event `EnhancedInput|/Game/Input/Actions/IA_Charge`
  (params (ActionValue :type Boolean) (ElapsedSeconds :type "Float (double-precision)") (TriggeredSeconds :type "Float (double-precision)") (InputAction :type "InputAction Object Reference" :default "/Game/Input/Actions/IA_Charge.IA_Charge"))
  ; INPUTS
  (:`Started`
    (`self.StartCharging`))
  (:`Completed`
    (`self.StopCharging`)))

(event `ChargeProgressionUpdate_Event`
  ; ChargingUpdate
  (if (`self.IsCharging`)
    (if (< (`self.CurrentFullyCharges`) (`self.MaxCharges`))
      ; Can Charge
      ;; Calcualte current progress
      (bind _output_get (set `self.CurrentChargeProgress` (`KismetMathLibrary.FClamp` (+ (* (`self.ChargingSpeed`) (`self.TicksPerChargeUpdate`)) (`self.CurrentChargeProgress`)))))
      ;; If current charge is not enought for new bullet, refresh progression, else change bullet count
      (if (>= _output_get 1.0)
        (set `self.CurrentChargeProgress` 0.0)
        (set `self.CurrentFullyCharges` (+ (`self.CurrentFullyCharges`) 1))
        (`/Game/UI/HUD/WBP_HUD.RefreshChargeCount` (`self.WBP_HUD`))
        ;; and check if we keep refreshing or stop charging
        (if (>= (`self.CurrentFullyCharges`) (`self.MaxCharges`))
          (`self.StopCharging`)
          (else
            (`/Game/UI/HUD/WBP_HUD.RefreshChargingProgression` (`self.WBP_HUD`))))
        (else
          (`/Game/UI/HUD/WBP_HUD.RefreshChargingProgression` (`self.WBP_HUD`))))
      (else
        (`self.StopCharging`)))))

(event `EnhancedInput|/Game/Input/Actions/IA_OpenPanel`
  (params (ActionValue :type Boolean) (ElapsedSeconds :type "Float (double-precision)") (TriggeredSeconds :type "Float (double-precision)") (InputAction :type "InputAction Object Reference" :default "/Game/Input/Actions/IA_OpenPanel.IA_OpenPanel"))
  ; INPUTS
  (:`Started`
    (`self.ShowPanel` true)))

(fn `ShowPanel`
  (params (showPanel :type Boolean))
  (bind _wbp_menu (`self.WBP_Menu`))
  (bind _output_get (set `self.OpenPanel` showPanel))
  (if _output_get
    (set `Widget.Visibility` "Hidden" (`self.WBP_HUD`))
    (set `Widget.Visibility` "Visible" (`self.WBP_Menu`))
    (`WidgetBlueprintLibrary.SetInputMode_UIOnlyEx` self (`self.WBP_Menu`))
    (set `self.bShowMouseCursor` true)
    (`CommonActivatableWidget.ActivateWidget` _wbp_menu)
    (else
      (set `Widget.Visibility` "Visible" (`self.WBP_HUD`))
      (set `Widget.Visibility` "Hidden" (`self.WBP_Menu`))
      (`WidgetBlueprintLibrary.SetInputMode_GameOnly` self)
      (set `self.bShowMouseCursor` false)
      (`CommonActivatableWidget.DeactivateWidget` _wbp_menu))))

(fn `StartCharging`
  (if (and (< (`self.CurrentFullyCharges`) (`self.MaxCharges`)) (not (`self.IsCharging`)))
    (set `self.IsCharging` true)
    (`/Game/UI/HUD/WBP_HUD.RefreshChargingState` (`self.WBP_HUD`))
    (`self.StartTimeEvent_Event`)))

(fn `StopCharging`
  (if (`self.IsCharging`)
    (set `self.IsCharging` false)
    (`/Game/UI/HUD/WBP_HUD.RefreshChargingState` (`self.WBP_HUD`))
    (`KismetSystemLibrary.K2_ClearAndInvalidateTimerHandle` (`self.ChargeTimerHandle`))))

(fn `UserConstructionScript`)